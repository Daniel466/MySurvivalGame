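; BP_ItemEquippableMaster is the base Blueprint for equippable items, handling equip state and use input.
; On the server it equips through ItemEquippableComp at BeginPlay and unequips when destroyed, so the actor's lifetime drives equip state.
; StartUse and StopUse forward to ItemUseComp's SERVER triggers.
; Getters expose its components, skeletal mesh, owning player character and hand IK transforms from a cached BPC_HandIK component.
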(event Custom|OnDestroyed_Event
  (params (DestroyedActor :type Actor%20Object%20Reference))
  ;[0.15 0.15 0.15 0.5] Initialization
  (Default|UnequipItem (Variables|Default|GetItemEquippableComp)))

(event EventBeginPlay
  ;[0.15 0.15 0.15 0.5] Initialization
  (|CallParentFunction)
  (Variables|Default|SetCachedHandIKComp (Actor|GetComponentbyClass "/Game/Core/Blueprints/Items/Components/BPC_HandIK.BPC_HandIK_C"))
  (Networking|SwitchHasAuthority
    (:Authority
      (Game|AssignOnDestroyed (delegate Custom|OnDestroyed_Event))
      (Default|EquipItem (Variables|Default|GetItemEquippableComp)))))

(event EventStartUse
  ;[0.15 0.15 0.15 0.5] Trigger to use items
  (Default|TriggerStartUseSERVER (Variables|Default|GetItemUseComp)))

(event EventStopUse
  ;[0.15 0.15 0.15 0.5] Trigger to use items
  (Default|TriggerStopUseSERVER (Variables|Default|GetItemUseComp)))

(fn ConstructionScript
  (|CallParentFunction))

(fn GetBpItemEquippable
  (return self))

(fn GetEquippedItemSkeletalMesh
  (return (Actor|GetComponentbyClass "/Script/Engine.SkeletalMeshComponent")))

(fn GetHandIKTransforms
  (bind _cachedhandikcomp (Variables|Default|GetCachedHandIKComp)
    (:then
      (return true (Default|GetLHIKTransform _cachedhandikcomp) (Default|GetRHIKTransform _cachedhandikcomp)))
    (:else)))

(fn GetItemEquippableComponent
  (return (Variables|Default|GetItemEquippableComp)))

(fn GetItemUseComponent
  (return (Variables|Default|GetItemUseComp)))

(fn GetOwningPlayerCharacter
  (bind _playercharacter (Class|BPICharacter|GetBpPlayerCharacter(Message) (Components|GetOwner)))
  (return _playercharacter))