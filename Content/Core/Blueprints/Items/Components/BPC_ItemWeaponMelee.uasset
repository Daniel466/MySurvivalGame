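; Melee weapon item component that plays the owning character's attack animation when the weapon is used.
; The weapon-used event calls a multicast event, which signals successful use and reads the equipment type from the item's data component.
; One-handed melee (axe montages) and spear each select a first- or third-person montage by active camera, played without a further multicast.
; The hardcoded montage selection is marked as testing only.
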(event Custom|ItemUsed_MULTICAST
  (bind _returnvalue (Components|GetOwner))
  (Default|CallOnWeaponUseSuccessfully)
  ;[0.9301 0 0 0.502] Just for testing
  (bind _playercharacter (Class|BPIItemEquippable|GetOwningPlayerCharacter(Message) _returnvalue))
  (bind _itemdatacomp (Class|BPIItemMaster|GetItemDataComp(Message) _returnvalue))
  (bind _itemequippabledata (Default|GetEquippableData _itemdatacomp))
  (switch Utilities|FlowControl|Switch|SwitchonE_ItemEquipmentType (Variables|/Game/Core/Blueprints/PrimaryDataAssets/Items/PDA_ItemEquippableMaster.PDA_ItemEquippableMaster_C|GetEquipmentType _itemequippabledata)
    (:NewEnumerator1
      (if (Variables|/Game/Core/Blueprints/Characters/BP_PlayerCharacter.BP_PlayerCharacter_C|GetIsFirstPersonCameraActive _playercharacter)
        (Class|BPICharacter|CharacterPlayAnimMontage(Message) _playercharacter false "/Game/Core/Art/Characters/PlayerCharacter/Animations/Equipment/Melee/M_Axe_FP_Attack_Montage.M_Axe_FP_Attack_Montage")
        (else
          (Class|BPICharacter|CharacterPlayAnimMontage(Message) _playercharacter false "/Game/Core/Art/Characters/PlayerCharacter/Animations/Equipment/Melee/M_Axe_TP_Attack_Montage.M_Axe_TP_Attack_Montage"))))
    (:NewEnumerator6
      (if (Variables|/Game/Core/Blueprints/Characters/BP_PlayerCharacter.BP_PlayerCharacter_C|GetIsFirstPersonCameraActive _playercharacter)
        (Class|BPICharacter|CharacterPlayAnimMontage(Message) _playercharacter false "/Game/Core/Art/Characters/PlayerCharacter/Animations/Equipment/Spear/M_Spear_FP_Attack_Montage.M_Spear_FP_Attack_Montage")
        (else
          (Class|BPICharacter|CharacterPlayAnimMontage(Message) _playercharacter false "/Game/Core/Art/Characters/PlayerCharacter/Animations/Equipment/Spear/M_Spear_TP_Attack_Montage.M_Spear_TP_Attack_Montage"))))))

(event EventHandleWeaponUsedEvent
  (CallFunction|ItemUsedMULTICAST))