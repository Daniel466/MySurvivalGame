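; Item component that runs server-side use of an equippable item in single, automatic or burst mode.
; When the item is equipped, it reads use mode, rate and burst count from the item's data.
; Starting use signals immediately, then a looping timer repeats it until the count runs out, use is stopped or the item becomes unusable.
; Bursts ignore stop requests, and restarting before a pending stop completes cancels that stop.
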(event Custom|OnItemEquipped_Event
  ;[0.15 0.15 0.15 0.5] Initialize Use Data
  (bind _itemdatacomp (Class|BPIItemMaster|GetItemDataComp(Message) (Components|GetOwner)))
  (bind _itemequippabledata (Default|GetEquippableData _itemdatacomp))
  (Variables|Default|SetUseInterval (/ 1.0 (Variables|/Game/Core/Blueprints/PrimaryDataAssets/Items/PDA_ItemEquippableMaster.PDA_ItemEquippableMaster_C|GetUseInterval _itemequippabledata)))
  (Variables|Default|SetCurrentUseMode (Variables|/Game/Core/Blueprints/PrimaryDataAssets/Items/PDA_ItemEquippableMaster.PDA_ItemEquippableMaster_C|GetUseMode _itemequippabledata))
  (Variables|Default|SetUseBurstCount (Variables|/Game/Core/Blueprints/PrimaryDataAssets/Items/PDA_ItemEquippableMaster.PDA_ItemEquippableMaster_C|GetUseBurstCount _itemequippabledata)))

(event Custom|TriggerStopUse_SERVER
  (if (Utilities|Enum|NotEqual(Enum) (Variables|Default|GetCurrentUseMode) "NewEnumerator2")
    (Variables|Default|SetShouldStopUsing true)))

(event Custom|TriggerStartUse_SERVER
  ;[0.15 0.15 0.15 0.5] Perform Usage
  (if (and (Variables|Default|GetShouldStopUsing) (Variables|Default|GetIsUsing))
    (Variables|Default|SetShouldStopUsing false)
    (elif (and (Variables|Default|GetIsUsable) (not (Variables|Default|GetIsUsing)))
      (Variables|Default|SetShouldStopUsing false)
      (Variables|Default|SetIsUsing true)
      (Default|CallOnItemUsed)
      (switch Utilities|FlowControl|Switch|SwitchonE_ItemUseMode (Variables|Default|GetCurrentUseMode)
        (:NewEnumerator0
          (CallFunction|StartUsingLoopTimer 1))
        (:NewEnumerator1
          (CallFunction|StartUsingLoopTimer 999))
        (:NewEnumerator2
          (CallFunction|StartUsingLoopTimer (Variables|Default|GetUseBurstCount)))))))

(event Custom|StartUsingLoopTimer
  (params (UsingLoopAmount :type Integer))
  ;[0.15 0.15 0.15 0.5] Timer for Burst/Automatic mode
  (Variables|Default|SetUsingCounter UsingLoopAmount)
  (bind _returnvalue (Utilities|Time|SetTimerbyEvent (delegate Custom|HandleItemUsing_Event) (Variables|Default|GetUseInterval) true))
  (Variables|Default|SetUseIntervalTimerRef _returnvalue))

(event Custom|HandleItemUsing_Event
  ;[0.15 0.15 0.15 0.5] Timer for Burst/Automatic mode
  (bind _result (Math|Integer|DecrementInt (Variables|Default|GetUsingCounter))
    (:%20%20
      (if (Math|Boolean|ANDBoolean (> _result 0) (Variables|Default|GetIsUsable) (not (Variables|Default|GetShouldStopUsing)))
        (Default|CallOnItemUsed)
        (else
          (CallFunction|ReadytoUseAgain))))))

(event Custom|ReadyToUseAgain
  (Default|CallOnItemUsedStop)
  (Variables|Default|SetIsUsing false)
  (Utilities|Time|ClearandInvalidateTimerbyHandle (Variables|Default|GetUseIntervalTimerRef)))

(event EventBeginPlay
  ;[0.15 0.15 0.15 0.5] Initialize Use Data
  (bind _itemequippablecomp (Class|BPIItemEquippable|GetItemEquippableComponent(Message) (Components|GetOwner)))
  (EventDispatchers|AssignOnItemEquipped _itemequippablecomp (delegate Custom|OnItemEquipped_Event)))

(event EventEndPlay
  (params (EndPlayReason :type EEndPlayReason%20Enum :default "Destroyed"))
  ;[0.15 0.15 0.15 0.5] Initialize Use Data
  (CallFunction|ReadytoUseAgain))