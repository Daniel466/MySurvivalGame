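; Item component that holds an item's data asset reference and gives access to its item data.
; The setter stores the soft reference, resolves it into a cached ItemData object and prints errors when the reference is invalid or fails to resolve.
; Equippable and resource getters query that cached object through message calls, returning each sub-data with a validity flag.
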(fn GetItemDataAsset
  (return (Variables|Default|GetItemDataAsset)))

(fn SetItemDataAsset
  (params (ItemDataAsset :type PDA%20Item%20Data%20Soft%20Object%20Reference))
  (Variables|Default|SetItemDataAsset ItemDataAsset)
  (if (Utilities|IsValidSoftObjectReference ItemDataAsset)
    (bind _itemdataasset (CallFunction|ResolveSoftItemDataReference (Variables|Default|GetItemDataAsset)))
    (bind _output_get (Variables|Default|SetItemData _itemdataasset))
    (Utilities|IsValid _output_get
      (:Is%20Not%20Valid
        _))
    (else
      (CallFunction|PrintError "ItemDataAsset is not valid in" (Utilities|GetDisplayName self) true)))
  (CallFunction|PrintError "ItemDataAsset Reference failed to Resolve in BP_ItemMaster" (Utilities|ToString(SoftObjectReference) (Variables|Default|GetItemDataAsset)) true))

(fn GetItemData
  (return (Variables|Default|GetItemData)))

(fn GetEquippableData
  (bind _itemequippabledata (Class|BPIAssets|GetItemEquippableData(Message) (Variables|Default|GetItemData)))
  (return (Utilities|IsValid _itemequippabledata) _itemequippabledata))

(fn GetResourceData
  (bind _itemresourcedata (Class|BPIAssets|GetItemResourceData(Message) (Variables|Default|GetItemData)))
  (return (Utilities|IsValid _itemresourcedata) _itemresourcedata))