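; PDA_ItemData is a primary data asset that serves as the base definition for game items, exposing their icon, stack information and a self reference through getters.
; An item counts as stackable when its stack size exceeds one, and IsItemStackable returns that flag together with the size.
; Durability defaults to none, with GetDefaultDurability meant for child classes to override.
; GetItemResource returns no value here.
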(fn IsStackable
  (return (> (Variables|Default|GetStackSize) 1)))

(fn GetDefaultDurability
  ;[0.4157 0.03137 0 0.502] Override function - used by children
  (return 0.0))

(fn GetIemIcon
  (return (Variables|Default|GetIcon)))

(fn GetItemData
  (return self))

(fn GetItemResource
  (return 0))

(fn IsItemDurabilityBased
  (return false))

(fn IsItemStackable
  (return (CallFunction|IsStackable) (Variables|Default|GetStackSize)))