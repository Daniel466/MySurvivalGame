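; Player character component that manages main-hand equipment, treating right-hand and two-handed slots alike.
; A server event destroys the current item, then async-loads and spawns the new item's actor class if its data asset is equippable.
; Slot assets are mirrored to the client by event, while the EquippedItemActor RepNotify broadcasts equip and unequip dispatchers.
; EndPlay unequips on authority when destroyed and unbinds both dispatchers.
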(event Custom|SetEquippedItem_SERVER
  (params (EquipmentSlot :type E_EquipmentSlot%20Enum :default "NewEnumerator0") (ItemDataAsset :type PDA%20Item%20Data%20Soft%20Object%20Reference))
  ;[0.15 0.15 0.15 0.5] Main Equipment event call
  (switch Utilities|FlowControl|Switch|SwitchonE_EquipmentSlot EquipmentSlot
    (:NewEnumerator1
      _)
    (:NewEnumerator2
      _))
  (CallFunction|UnequipMainHandItem "NewEnumerator1")
  (CallFunction|SpawnMainHandItem EquipmentSlot ItemDataAsset))

(event Custom|UnequipMainHandItem
  (params (EquipmentSlot :type E_EquipmentSlot%20Enum :default "NewEnumerator0"))
  ;[0.15 0.15 0.15 0.5] Handle MainHand Equipment
  (bind _equippeditemactor (Variables|Default|GetEquippedItemActor)
    (:then
      (Actor|DestroyActor _equippeditemactor)
      (Variables|Default|SetEquippedItemActor 0)
      (CallFunction|SetEquipmentSlotAsset EquipmentSlot))
    (:else)))

(event Custom|SetEquipmentSlotAsset_CLIENT
  (params (EquipmentSlot :type E_EquipmentSlot%20Enum%20%28by%20ref%29 :default "NewEnumerator0") (ItemDataAsset :type PDA%20Item%20Data%20Soft%20Object%20Reference%20%28by%20ref%29))
  ;[0.15 0.15 0.15 0.5] Replicate the EquipmentSlots Map to the client
  (Utilities|Map|Add (Variables|Default|GetEquipmentSlots) EquipmentSlot ItemDataAsset))

(event Custom|SetEquipmentSlotAsset
  (params (EquipmentSlot :type E_EquipmentSlot%20Enum%20%28by%20ref%29 :default "NewEnumerator0") (ItemDataAsset :type PDA%20Item%20Data%20Soft%20Object%20Reference%20%28by%20ref%29))
  ;[0.15 0.15 0.15 0.5] Replicate the EquipmentSlots Map to the client
  (Utilities|Map|Add (Variables|Default|GetEquipmentSlots) EquipmentSlot ItemDataAsset)
  (CallFunction|SetEquipmentSlotAssetCLIENT "NewEnumerator0"))

(event Custom|SpawnMainHandItem
  (params (EquipmentSlot :type E_EquipmentSlot%20Enum :default "NewEnumerator0") (ItemDataAsset :type PDA%20Item%20Data%20Soft%20Object%20Reference))
  (bind _playercharacter (Variables|Default|GetPlayerCharacter))
  ;[0.15 0.15 0.15 0.5] Handle MainHand Equipment
  (if (Utilities|IsValidSoftObjectReference ItemDataAsset)
    (bind _itemdataasset (CallFunction|ResolveSoftItemDataReference ItemDataAsset))
    (bind _itemequippabledata (Class|BPIAssets|GetItemEquippableData(Message) _itemdataasset))
    (bind _returnvalue (Class|BPIItemData|IsItemEquippable(Message) _itemequippabledata))
    (if _returnvalue
      (CallFunction|SetEquipmentSlotAsset EquipmentSlot ItemDataAsset)
      (Utilities|AsyncLoadClassAsset (Variables|/Game/Core/Blueprints/PrimaryDataAssets/Items/PDA_ItemEquippableMaster.PDA_ItemEquippableMaster_C|GetEquipActorClass _itemequippabledata)
        (:Completed
          (bind _returnvalue_2 (Game|SpawnActorfromClass (Utilities|ResolveSoftReference (Variables|/Game/Core/Blueprints/PrimaryDataAssets/Items/PDA_ItemEquippableMaster.PDA_ItemEquippableMaster_C|GetEquipActorClass _itemequippabledata)) (Math|Transform|MakeTransform "0, 0, 0" "0, 0, 0" "1.000000,1.000000,1.000000") "AlwaysSpawn" "MultiplyWithRoot" _playercharacter ItemDataAsset _playercharacter))
          (Variables|Default|SetEquippedItemActor _returnvalue_2))))))

(event EventBeginPlay
  ;[0.15 0.15 0.15 0.5] Begin Play
  (bind _playercharacter (Class|BPICharacter|GetPlayerCharacterRef(Message) (Components|GetOwner)))
  (Variables|Default|SetPlayerCharacter _playercharacter))

(event EventEndPlay
  (params (EndPlayReason :type EEndPlayReason%20Enum :default "Destroyed"))
  ;[0.15 0.15 0.15 0.5] If player disconnect, cleanup equipments
  (Utilities|FlowControl|Sequence
    (:then_0
      (Networking|SwitchHasAuthority
        (:Authority
          (switch Utilities|FlowControl|Switch|SwitchonEEndPlayReason EndPlayReason
            (:Destroyed
              (CallFunction|UnequipMainHandItem "NewEnumerator1"))))))
    (:then_1
      (EventDispatchers|UnbindallEventsfromOnMainHandEquipped)
      (EventDispatchers|UnbindallEventsfromOnMainHandUnequipped))))

(fn OnRepEquippedItemActor
  (bind _equippeditemactor (Variables|Default|GetEquippedItemActor)
    (:then
      (Default|CallOnMainHandEquipped _equippeditemactor))
    (:else
      (Default|CallOnMainHandUnequipped))))