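; Player hotbar inventory component that selects slots by number key or scroll and requests equip or unequip through SERVER events.
; Hotkeys act immediately, while scrolling skips empty slots and debounces with a retriggerable delay; reselecting the equipped slot unequips it.
; On slot changes, authority re-equips a changed equipped item and remotes rebroadcast the selection highlight.
; Equip and unequip currently only track slot state and print TODOs, without touching the character.
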(event Custom|SetSelectedSlotIndex
  (params (SelectedSlotIndex :type Integer))
  ;[0.15 0.15 0.15 0.5] Hotbar selection & scroll
  (bind _output_get (Variables|Default|SetCurrentScrollIndex SelectedSlotIndex))
  (bind _output_get_2 (Variables|Default|SetSelectedSlotIndex _output_get))
  (bind _hasitem (CallFunction|TryGetSlotItemDataAsset _output_get_2))
  (Default|CallOnHarbarSlotSelected _hasitem _output_get_2)
  (Variables|Default|SetIsHotkeyPressed true)
  (if (== (Variables|Default|GetEquippedHotbarSlotIndex) (Variables|Default|GetSelectedSlotIndex))
    (CallFunction|UnequipCurrentItemSERVER)
    ;[0.15 0.15 0.15 0.5] Not Equippable items, Highlighted all time
    (bind _itemdataasset (CallFunction|TryGetSlotItemDataAsset (Variables|Default|GetSelectedSlotIndex)))
    (bind _itemdataasset_2 (CallFunction|ResolveSoftItemDataReference _itemdataasset))
    (bind _returnvalue (Class|BPIItemData|IsItemEquippable(Message) _itemdataasset_2))
    (Default|CallOnHarbarSlotSelected (not _returnvalue) (Variables|Default|GetSelectedSlotIndex))
    (else
      (CallFunction|TrytoEquipItemSERVER (Variables|Default|GetSelectedSlotIndex)))))

(event Custom|UnequipCurrentItem_SERVER
  ;[0.15 0.15 0.15 0.5] Equip / Unequip items on character
  (bind _output_get (Variables|Default|SetEquippedHotbarSlotIndex -1))
  (CallFunction|PrintTodo "Unequip Slot Index" (Utilities|String|ToString(Integer) _output_get) true))

(event Custom|TryToEquipItem_SERVER
  (params (SlotIndex :type Integer))
  ;[0.15 0.15 0.15 0.5] Equip / Unequip items on character
  (bind _output_get (Variables|Default|SetEquippedHotbarSlotIndex SlotIndex))
  (bind _itemdataasset (CallFunction|TryGetSlotItemDataAsset _output_get))
  (Variables|Default|SetEquippedItemDataAsset _itemdataasset)
  (CallFunction|PrintTodo "Try to equip item SlotIndex" (Utilities|String|Append (Utilities|String|ToString(Integer) _output_get) " Asset: " (Utilities|String|ToString(Integer) _output_get)) true))

(event Custom|SetSelectedSlotIndexByScroll
  (params (SelectedSlotIndex :type Integer))
  ;[0.15 0.15 0.15 0.5] Hotbar selection & scroll
  (bind _output_get (Variables|Default|SetSelectedSlotIndex SelectedSlotIndex))
  (Default|CallOnHarbarSlotSelected true _output_get)
  (Variables|Default|SetIsHotkeyPressed false)
  (Utilities|FlowControl|RetriggerableDelay 0.15)
  (if (not (Variables|Default|GetIsHotkeyPressed))
    (if (== (Variables|Default|GetEquippedHotbarSlotIndex) (Variables|Default|GetSelectedSlotIndex))
      (CallFunction|UnequipCurrentItemSERVER)
      ;[0.15 0.15 0.15 0.5] Not Equippable items, Highlighted all time
      (bind _itemdataasset (CallFunction|TryGetSlotItemDataAsset (Variables|Default|GetSelectedSlotIndex)))
      (bind _itemdataasset_2 (CallFunction|ResolveSoftItemDataReference _itemdataasset))
      (bind _returnvalue (Class|BPIItemData|IsItemEquippable(Message) _itemdataasset_2))
      (Default|CallOnHarbarSlotSelected (not _returnvalue) (Variables|Default|GetSelectedSlotIndex))
      (else
        (CallFunction|TrytoEquipItemSERVER (Variables|Default|GetSelectedSlotIndex))))))

(event Custom|OnSlotChanged_Event
  (params (Slot :type S%20Inventory%20Slot%20Structure))
  ;[0.15 0.15 0.15 0.5] On slot changed reaction
  (if (== (Variables|Default|GetEquippedHotbarSlotIndex) (Utilities|Struct|BreakS_InventorySlot Slot))
    (Default|CallOnHarbarSlotSelected (CallFunction|IsSlotNotEmpty Slot) (Variables|Default|GetEquippedHotbarSlotIndex))))

(event Custom|OnSlotChanged_Event_0
  (params (Slot :type S%20Inventory%20Slot%20Structure))
  (bind (_slotindex _itemdataasset) (Utilities|Struct|BreakS_InventorySlot Slot))
  ;[0.15 0.15 0.15 0.5] On slot changed reaction
  (if (and (== (Variables|Default|GetEquippedHotbarSlotIndex) _slotindex) (!= _itemdataasset (Variables|Default|GetEquippedItemDataAsset)))
    (CallFunction|TrytoEquipItemSERVER _slotindex)))

(event Input|EnhancedActionEvents|EnhancedInputActionIA_Hotbar_00
  (params (ActionValue :type Boolean) (ElapsedSeconds :type Float%20%28double-precision%29) (TriggeredSeconds :type Float%20%28double-precision%29) (InputAction :type Input%20Action%20Object%20Reference :default "/Game/Core/Data/Input/Actions/Hotbar/IA_Hotbar_00.IA_Hotbar_00"))
  ;[0.15 0.15 0.15 0.5] Hotbar keys
  (CallFunction|SetSelectedSlotIndex 9))

(event Input|EnhancedActionEvents|EnhancedInputActionIA_Hotbar_02
  (params (ActionValue :type Boolean) (ElapsedSeconds :type Float%20%28double-precision%29) (TriggeredSeconds :type Float%20%28double-precision%29) (InputAction :type Input%20Action%20Object%20Reference :default "/Game/Core/Data/Input/Actions/Hotbar/IA_Hotbar_02.IA_Hotbar_02"))
  ;[0.15 0.15 0.15 0.5] Hotbar keys
  (CallFunction|SetSelectedSlotIndex 1))

(event Input|EnhancedActionEvents|EnhancedInputActionIA_Hotbar_09
  (params (ActionValue :type Boolean) (ElapsedSeconds :type Float%20%28double-precision%29) (TriggeredSeconds :type Float%20%28double-precision%29) (InputAction :type Input%20Action%20Object%20Reference :default "/Game/Core/Data/Input/Actions/Hotbar/IA_Hotbar_09.IA_Hotbar_09"))
  ;[0.15 0.15 0.15 0.5] Hotbar keys
  (CallFunction|SetSelectedSlotIndex 8))

(event Input|EnhancedActionEvents|EnhancedInputActionIA_Hotbar_ScrollRight
  (params (ActionValue :type Boolean) (ElapsedSeconds :type Float%20%28double-precision%29) (TriggeredSeconds :type Float%20%28double-precision%29) (InputAction :type Input%20Action%20Object%20Reference :default "/Game/Core/Data/Input/Actions/Hotbar/IA_Hotbar_ScrollRight.IA_Hotbar_ScrollRight"))
  ;[0.15 0.15 0.15 0.5] Hotbar selection & scroll
  (CallFunction|RotateHotbarSlotIndex 1))

(event Input|EnhancedActionEvents|EnhancedInputActionIA_Hotbar_ScrollLeft
  (params (ActionValue :type Boolean) (ElapsedSeconds :type Float%20%28double-precision%29) (TriggeredSeconds :type Float%20%28double-precision%29) (InputAction :type Input%20Action%20Object%20Reference :default "/Game/Core/Data/Input/Actions/Hotbar/IA_Hotbar_ScrollLeft.IA_Hotbar_ScrollLeft"))
  ;[0.15 0.15 0.15 0.5] Hotbar selection & scroll
  (CallFunction|RotateHotbarSlotIndex -1))

(event Input|EnhancedActionEvents|EnhancedInputActionIA_Hotbar_01
  (params (ActionValue :type Boolean) (ElapsedSeconds :type Float%20%28double-precision%29) (TriggeredSeconds :type Float%20%28double-precision%29) (InputAction :type Input%20Action%20Object%20Reference :default "/Game/Core/Data/Input/Actions/Hotbar/IA_Hotbar_01.IA_Hotbar_01"))
  ;[0.15 0.15 0.15 0.5] Hotbar keys
  (CallFunction|SetSelectedSlotIndex))

(event Input|EnhancedActionEvents|EnhancedInputActionIA_Hotbar_03
  (params (ActionValue :type Boolean) (ElapsedSeconds :type Float%20%28double-precision%29) (TriggeredSeconds :type Float%20%28double-precision%29) (InputAction :type Input%20Action%20Object%20Reference :default "/Game/Core/Data/Input/Actions/Hotbar/IA_Hotbar_03.IA_Hotbar_03"))
  ;[0.15 0.15 0.15 0.5] Hotbar keys
  (CallFunction|SetSelectedSlotIndex 2))

(event Input|EnhancedActionEvents|EnhancedInputActionIA_Hotbar_04
  (params (ActionValue :type Boolean) (ElapsedSeconds :type Float%20%28double-precision%29) (TriggeredSeconds :type Float%20%28double-precision%29) (InputAction :type Input%20Action%20Object%20Reference :default "/Game/Core/Data/Input/Actions/Hotbar/IA_Hotbar_04.IA_Hotbar_04"))
  ;[0.15 0.15 0.15 0.5] Hotbar keys
  (CallFunction|SetSelectedSlotIndex 3))

(event Input|EnhancedActionEvents|EnhancedInputActionIA_Hotbar_05
  (params (ActionValue :type Boolean) (ElapsedSeconds :type Float%20%28double-precision%29) (TriggeredSeconds :type Float%20%28double-precision%29) (InputAction :type Input%20Action%20Object%20Reference :default "/Game/Core/Data/Input/Actions/Hotbar/IA_Hotbar_05.IA_Hotbar_05"))
  ;[0.15 0.15 0.15 0.5] Hotbar keys
  (CallFunction|SetSelectedSlotIndex 4))

(event Input|EnhancedActionEvents|EnhancedInputActionIA_Hotbar_06
  (params (ActionValue :type Boolean) (ElapsedSeconds :type Float%20%28double-precision%29) (TriggeredSeconds :type Float%20%28double-precision%29) (InputAction :type Input%20Action%20Object%20Reference :default "/Game/Core/Data/Input/Actions/Hotbar/IA_Hotbar_06.IA_Hotbar_06"))
  ;[0.15 0.15 0.15 0.5] Hotbar keys
  (CallFunction|SetSelectedSlotIndex 5))

(event Input|EnhancedActionEvents|EnhancedInputActionIA_Hotbar_07
  (params (ActionValue :type Boolean) (ElapsedSeconds :type Float%20%28double-precision%29) (TriggeredSeconds :type Float%20%28double-precision%29) (InputAction :type Input%20Action%20Object%20Reference :default "/Game/Core/Data/Input/Actions/Hotbar/IA_Hotbar_07.IA_Hotbar_07"))
  ;[0.15 0.15 0.15 0.5] Hotbar keys
  (CallFunction|SetSelectedSlotIndex 6))

(event Input|EnhancedActionEvents|EnhancedInputActionIA_Hotbar_08
  (params (ActionValue :type Boolean) (ElapsedSeconds :type Float%20%28double-precision%29) (TriggeredSeconds :type Float%20%28double-precision%29) (InputAction :type Input%20Action%20Object%20Reference :default "/Game/Core/Data/Input/Actions/Hotbar/IA_Hotbar_08.IA_Hotbar_08"))
  ;[0.15 0.15 0.15 0.5] Hotbar keys
  (CallFunction|SetSelectedSlotIndex 7))

(event EventBeginPlay
  ;[0.15 0.15 0.15 0.5] Begin play
  (|CallParentFunction)
  (bind _playercharacter (Class|BPICharacter|GetPlayerCharacterRef(Message) (Components|GetOwner)))
  (Variables|References|SetPlayerCharacter _playercharacter)
  ;[0.15 0.15 0.15 0.5] On slot changed reaction
  (Networking|SwitchHasAuthority
    (:Authority
      (EventDispatchers|BindEventtoOnSlotChanged (delegate Custom|OnSlotChanged_Event_0)))
    (:Remote
      (EventDispatchers|AssignOnSlotChanged (delegate Custom|OnSlotChanged_Event)))))

(event EventEndPlay
  (params (EndPlayReason :type EEndPlayReason%20Enum :default "Destroyed"))
  ;[0.15 0.15 0.15 0.5] Begin play
  (EventDispatchers|UnbindallEventsfromOnHarbarSlotSelected))

(fn TryGetSlotItemDataAsset
  (params (Index :type Integer))
  (bind (_isvalid _slot) (CallFunction|GetSlotatIndex Index))
  (if (and _isvalid (CallFunction|IsSlotEmpty _slot))
    (return false 0)
    (else
      (return true (Utilities|Struct|BreakS_InventorySlot _slot)))))

(fn RotateHotbarSlotIndex
  (params (ScrollDirection :type Integer))
  (Utilities|FlowControl|ForLoopwithBreak 0 (Variables|Default|GetMaxSlotCount) :!label _label
    (:LoopBody
      (bind _output_get (Variables|Default|SetCurrentScrollIndex (+ (Variables|Default|GetCurrentScrollIndex) ScrollDirection)))
      (if (>= _output_get (Variables|Default|GetMaxSlotCount))
        (Variables|Default|SetCurrentScrollIndex 0)
        (elif (< (Variables|Default|GetCurrentScrollIndex) 0)
          (bind _output_get_2 (Variables|Default|SetCurrentScrollIndex (- (Variables|Default|GetMaxSlotCount) 1)))))
      (bind _hasitem (CallFunction|TryGetSlotItemDataAsset _output_get_2))
      (if _hasitem
        (LocalVariables|SetSlotFound true)
        (goto _label Break)))
    (:Completed
      (if (LocalVariables|GetSlotFound)
        (CallFunction|SetSelectedSlotIndexbyScroll (Variables|Default|GetCurrentScrollIndex))))))