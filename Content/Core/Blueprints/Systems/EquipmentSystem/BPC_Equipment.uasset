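; Equipment component that handles equipping and unequipping the player's main-hand item in a replicated setup.
; The server equip event destroys the current item, records the new item asset in a slot map mirrored to the client, then async-loads and spawns its actor; both-hands items share the right-hand path.
; The equipped actor's OnRep broadcasts arm pose, attach socket and equip or unequip events, defaulting to an unarmed pose.
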(event Custom|SetEquippedItem_SERVER
  (params (EquipmentSlot :type E_ItemEquipmentSlot%20Enum :default "NewEnumerator0") (ItemDataAsset :type PDA%20Item%20Data%20Soft%20Object%20Reference))
  ;[0.15 0.15 0.15 0.5] Main Equipment event call
  (switch Utilities|FlowControl|Switch|SwitchonE_ItemEquipmentSlot EquipmentSlot
    (:NewEnumerator1
      _)
    (:NewEnumerator2
      _))
  (CallFunction|UnequipMainHandItem "NewEnumerator1")
  (CallFunction|SpawnMainHandItem "NewEnumerator1" ItemDataAsset))

(event Custom|SetEquipmentSlotAsset_CLIENT
  (params (EquipmentSlot :type E_ItemEquipmentSlot%20Enum%20%28by%20ref%29 :default "NewEnumerator0") (ItemDataAsset :type PDA%20Item%20Data%20Soft%20Object%20Reference%20%28by%20ref%29))
  ;[0.15 0.15 0.15 0.5] Replicate the EquipmentSlots Map to the client
  (Utilities|Map|Add (Variables|Default|GetEquipmentSlots) EquipmentSlot ItemDataAsset))

(event Custom|SetEquipmentSlotAsset
  (params (EquipmentSlot :type E_ItemEquipmentSlot%20Enum%20%28by%20ref%29 :default "NewEnumerator0") (ItemDataAsset :type PDA%20Item%20Data%20Soft%20Object%20Reference%20%28by%20ref%29))
  ;[0.15 0.15 0.15 0.5] Replicate the EquipmentSlots Map to the client
  (Utilities|Map|Add (Variables|Default|GetEquipmentSlots) EquipmentSlot ItemDataAsset)
  (CallFunction|SetEquipmentSlotAssetCLIENT "NewEnumerator0"))

(event Custom|SpawnMainHandItem
  (params (EquipmentSlot :type E_ItemEquipmentSlot%20Enum :default "NewEnumerator0") (ItemDataAsset :type PDA%20Item%20Data%20Soft%20Object%20Reference))
  ;[0.15 0.15 0.15 0.5] Handle MainHand Equipment
  (if (Utilities|IsValidSoftObjectReference ItemDataAsset)
    (bind _itemdataasset (CallFunction|ResolveSoftItemDataReference ItemDataAsset))
    (bind _itemequippabledata (Class|BPIAssets|GetItemEquippableData(Message) _itemdataasset))
    (bind _returnvalue (Class|BPIItemData|IsItemEquippable(Message) _itemequippabledata))
    (if _returnvalue
      (CallFunction|SetEquipmentSlotAsset EquipmentSlot ItemDataAsset)
      (bind _playercharacter (Class|BPICharacter|GetBpPlayerCharacter(Message) (Components|GetOwner)))
      (Utilities|AsyncLoadClassAsset (Variables|/Game/Core/Blueprints/PrimaryDataAssets/Items/PDA_ItemEquippableMaster.PDA_ItemEquippableMaster_C|GetEquipActorClass _itemequippabledata)
        (:Completed
          (bind _returnvalue_2 (Game|SpawnActorfromClass (Utilities|ResolveSoftReference (Variables|/Game/Core/Blueprints/PrimaryDataAssets/Items/PDA_ItemEquippableMaster.PDA_ItemEquippableMaster_C|GetEquipActorClass _itemequippabledata)) (Math|Transform|MakeTransform "0, 0, 0" "0, 0, 0" "1.000000,1.000000,1.000000") "AlwaysSpawn" "MultiplyWithRoot" _playercharacter ItemDataAsset _playercharacter))
          (Variables|Default|SetEquippedItemActor _returnvalue_2))))))

(event EventEndPlay
  (params (EndPlayReason :type EEndPlayReason%20Enum :default "Destroyed"))
  ;[0.15 0.15 0.15 0.5] If player disconnect, cleanup equipments
  (Utilities|FlowControl|Sequence
    (:then_0
      (Networking|SwitchHasAuthority
        (:Authority
          (switch Utilities|FlowControl|Switch|SwitchonEEndPlayReason EndPlayReason
            (:Destroyed
              (CallFunction|UnequipMainHandItem "NewEnumerator1"))))))
    (:then_1
      (EventDispatchers|UnbindallEventsfromOnMainHandEquipped)
      (EventDispatchers|UnbindallEventsfromOnMainHandUnequipped))))

(fn UnequipMainHandItem
  (params (EquipmentSlot :type E_ItemEquipmentSlot%20Enum :default "NewEnumerator0"))
  (bind _equippeditemactor (Variables|Default|GetEquippedItemActor)
    (:then
      (Actor|DestroyActor _equippeditemactor)
      (Variables|Default|SetEquippedItemActor 0)
      (CallFunction|SetEquipmentSlotAsset EquipmentSlot))
    (:else)))

(fn OnRepEquippedItemActor
  (bind (_armposeasset _attachsocket) (EquipmentComponent|GetEquippedMainHandArmPoseSet))
  (Default|CallOnArmPoseSetChange _armposeasset _attachsocket)
  (bind _equippeditemactor (Variables|Default|GetEquippedItemActor)
    (:then
      (Default|CallOnMainHandEquipped _equippeditemactor))
    (:else
      (Default|CallOnMainHandUnequipped))))

(fn GetEquippedMainHandActor
  (return (Variables|Default|GetEquippedItemActor)))

(fn GetEquippedSlotItemDataAsset
  (params (EquipmentSlot :type E_ItemEquipmentSlot%20Enum :default "NewEnumerator0"))
  (bind _equipmentslots (Variables|Default|GetEquipmentSlots))
  (bind _value (Utilities|Map|Find _equipmentslots EquipmentSlot))
  (return (Utilities|IsValidSoftObjectReference _value) _value))

(fn GetEquippedMainHandArmPoseSet
  (bind _equippeditemactor (Variables|Default|GetEquippedItemActor)
    (:then
      (bind _itemdatacomp (Default|GetItemDataComp _equippeditemactor))
      (bind (_isvalid _itemequippabledata) (Default|GetEquippableData _itemdatacomp))
      (if _isvalid
        (return (Variables|/Game/Core/Blueprints/PrimaryDataAssets/Items/PDA_ItemEquippableMaster.PDA_ItemEquippableMaster_C|GetArmPoseAsset _itemequippabledata) (Variables|/Game/Core/Blueprints/PrimaryDataAssets/Items/PDA_ItemEquippableMaster.PDA_ItemEquippableMaster_C|GetAttachSocket _itemequippabledata))
        (else
          _)))
    (:else
      _))
  (return "/Game/Core/DataAssets/ArmPoseSets/DA_ArmPoseSet_Unarmed.DA_ArmPoseSet_Unarmed" "NewEnumerator0"))

(fn IsMainHandEquipped
  (Variables|Default|GetEquippedItemActor
    (:then
      (return true))
    (:else
      (return false))))