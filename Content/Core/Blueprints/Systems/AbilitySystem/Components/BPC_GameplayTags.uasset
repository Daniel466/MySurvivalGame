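; Gameplay tag component for the ability system that holds a replicated set of active tags, with exact-match queries.
; Set events add or remove tags without duplicates, then pass previous and current containers to a diff routine, which OnRep also runs on clients.
; Each reported change fires an any-tag dispatcher and messages objects bound to that tag, with an empty listener container matching every tag.
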(event Custom|SetGameplayTags
  (params (Tags :type Gameplay%20Tag%20Container%20Structure) (Enabled :type Boolean))
  ;[0.15 0.15 0.15 0.5] Set Gameplay Tag States
  (CallFunction|UpdateTagState Tags Enabled))

(event Custom|SetGameplayTag
  (params (Tag :type Gameplay%20Tag%20Structure) (Enabled :type Boolean))
  ;[0.15 0.15 0.15 0.5] Set Gameplay Tag States
  (CallFunction|UpdateTagState (GameplayTags|MakeGameplayTagContainerfromTag Tag) Enabled))

(fn UpdateTagState
  (params (Tags :type Gameplay%20Tag%20Container%20Structure) (Enabled :type Boolean))
  ;[0.15 0.15 0.15 0.5] Adds or removes the tags based on the Enabled value, prevents duplicated, and notifies listeners via ProcessTagDiffAndNotify
  (Variables|GameplayTagsComponent|SetPreActiveTags (Variables|GameplayTagsComponent|GetActiveTags))
  (for _array_element (GameplayTags|BreakGameplayTagContainer Tags)
    (if Enabled
      (if (not (GameplayTagsComponent|HasActiveTag _array_element))
        (GameplayTags|AddGameplayTag (Variables|GameplayTagsComponent|GetActiveTags) _array_element :!class /Script/GameplayTags.BlueprintGameplayTagLibrary))
      (elif (GameplayTagsComponent|HasActiveTag _array_element)
        (GameplayTags|RemoveGameplayTag (Variables|GameplayTagsComponent|GetActiveTags) _array_element :!class /Script/GameplayTags.BlueprintGameplayTagLibrary))))
  (CallFunction|ProcessTagDiffandNotify (Variables|GameplayTagsComponent|GetPreActiveTags) (Variables|GameplayTagsComponent|GetActiveTags)))

(fn HasActiveTag
  (params (Tag :type Gameplay%20Tag%20Structure))
  ;[0.15 0.15 0.15 0.5] Checks if the provided tag exists in the list of currently active tags.
  ; Uses exact match to ensure the tag must be present without partial hierarchy inclusion.
  (return (GameplayTags|HasTag (Variables|GameplayTagsComponent|GetActiveTags) Tag true)))

(fn HasActiveTags
  (params (Tags :type Gameplay%20Tag%20Container%20Structure) (AllTags :type Boolean))
  ;[0.15 0.15 0.15 0.5] Returns true if the specified tag or any tag from the input container exists in the list of active tags.
  ; Use the 'All Tags' input to require all tags to be present instead of just one.
  (if AllTags
    (return (GameplayTags|HasAllTags (Variables|GameplayTagsComponent|GetActiveTags) Tags true))
    (else
      (return (GameplayTags|HasAnyTags (Variables|GameplayTagsComponent|GetActiveTags) Tags true)))))

(fn NotifyLocalTagChanged
  (params (TagChangedContext :type S%20Gameplay%20Tag%20Changed%20Context%20Structure))
  ;[0.15 0.15 0.15 0.5] Iterates through all registered listeners and checks if the given tag matches any stored listener entry.
  ; If a match is found and the tag state changed, the listener is notifed with the updated tag value and the associated gameplay effect context.
  (Default|CallOnAnyTagChanged TagChangedContext)
  (bind _keys (Utilities|Map|Keys (Variables|GameplayTagsComponentListener|GetTagsListener)))
  (for _array_element _keys
    (if (.ReturnValue (Utilities|Map|Find (Variables|GameplayTagsComponentListener|GetTagsListener) _array_element))
      (if (or (CallFunction|IsTagContainerEmpty (.Value (Utilities|Map|Find (Variables|GameplayTagsComponentListener|GetTagsListener) _array_element))) (GameplayTags|HasTag (.Value (Utilities|Map|Find (Variables|GameplayTagsComponentListener|GetTagsListener) _array_element)) (Utilities|Struct|BreakS_GameplayTagChangedContext TagChangedContext) true))
        (Class|BPIGameplayTagListener|OnTagChanged(Message) _array_element TagChangedContext)))))

(fn ProcessTagDiffandNotify
  (params (PrevContainer :type Gameplay%20Tag%20Container%20Structure) (NewContainer :type Gameplay%20Tag%20Container%20Structure))
  ;[0.15 0.15 0.15 0.5] Compares the previous and current Gameplay Tag Containers and identifies which tags were added or removed.
  ; Each change is processed individually by invoking the HandleLocalTagChanged function.
  ; This allows local tag listeners to react precisely to changes in the active tag set.
  (Variables|GameplayTagsComponent|SetPreActiveTags NewContainer)
  (LocalVariables|SetTagChangedContext (Utilities|Struct|MakeS_GameplayTagChangedContext "(TagName=\"\")" NewContainer false))
  (for _array_element (GameplayTags|BreakGameplayTagContainer NewContainer)
    (bind _returnvalue (GameplayTags|RemoveGameplayTag PrevContainer _array_element :!class /Script/GameplayTags.BlueprintGameplayTagLibrary))
    (if _returnvalue
      (bind _structout (Utilities|Struct|SetmembersinS_GameplayTagChangedContext (LocalVariables|GetTagChangedContext) _array_element true))
      (CallFunction|NotifyLocalTagChanged _structout)))
  (for _array_element_2 (GameplayTags|BreakGameplayTagContainer (Variables|GameplayTagsComponent|GetPreActiveTags))
    (bind _structout_2 (Utilities|Struct|SetmembersinS_GameplayTagChangedContext (LocalVariables|GetTagChangedContext) _array_element_2 false))
    (CallFunction|NotifyLocalTagChanged _structout_2)))

(fn OnRepActiveTags
  ;[0.15 0.15 0.15 0.5] Called on clients when the replicated ActiveTags array is updated.
  ; Triggers local tag change processing and notifies listeners by comparing the previous and current state.
  (CallFunction|ProcessTagDiffandNotify (Variables|GameplayTagsComponent|GetPreActiveTags) (Variables|GameplayTagsComponent|GetActiveTags)))

(fn BindTagListener
  (params (ListenerObject :type Object%20Object%20Reference) (Tags :type Gameplay%20Tag%20Container%20Structure))
  (bind _tagslistener (Variables|GameplayTagsComponentListener|GetTagsListener))
  (bind (_value _returnvalue) (Utilities|Map|Find _tagslistener ListenerObject))
  ;[0.15 0.15 0.15 0.5] Binds a listener to tag changes while preventing duplicated.
  ; If a listener for this target already exists, the new tags are added to it's container instead of creating a duplicate entry.
  (LocalVariables|SetTagContainer (select _returnvalue _value ""))
  (for _array_element (GameplayTags|BreakGameplayTagContainer Tags)
    (GameplayTags|AddGameplayTag (LocalVariables|GetTagContainer) _array_element :!class /Script/GameplayTags.BlueprintGameplayTagLibrary))
  (Utilities|Map|Add (Variables|GameplayTagsComponentListener|GetTagsListener) ListenerObject (LocalVariables|GetTagContainer)))

(fn UnbindListenerfromAllTags
  (params (ListenerObject :type Object%20Object%20Reference))
  (Utilities|Map|Remove (Variables|GameplayTagsComponentListener|GetTagsListener) ListenerObject))

(fn GetActiveTags
  (return (Variables|GameplayTagsComponent|GetActiveTags)))