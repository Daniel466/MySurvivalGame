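; BPC_AbilitySystem is an actor component that gives access to the owner's ability-related components and gameplay tags.
; It returns itself as the ability system and fetches the attribute system and gameplay tags components through messages to its owner.
; Tag queries and changes are forwarded to the gameplay tags component.
; It holds no ability logic in these graphs, and BeginPlay and Tick are unused.
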(event EventBeginPlay)

(event EventTick
  (params (DeltaSeconds :type Float%20%28single-precision%29)))

(fn GetAbilitySystemComp
  (return self))

(fn GetAttributeSystemComp
  (bind _attributesystemcomp (Class|BPIAbilitySystemProvider|GetAttributeSystemComp(Message) (Components|GetOwner)))
  (return _attributesystemcomp))

(fn GetGameplayTagsComp
  (bind _gameplaytagcomp (Class|BPIAbilitySystemProvider|GetGameplayTagsComp(Message) (Components|GetOwner)))
  (return _gameplaytagcomp))

(fn HasGameplayTag
  (params (Tag :type Gameplay%20Tag%20Structure))
  (bind _gameplaytagcomp (CallFunction|GetGameplayTagsComp))
  (bind _result (Default|HasActiveTag _gameplaytagcomp Tag))
  (return _result))

(fn SetGameplayTag
  (params (Tag :type Gameplay%20Tag%20Structure) (Active :type Boolean))
  (bind _gameplaytagcomp (CallFunction|GetGameplayTagsComp))
  (Default|SetGameplayTag _gameplaytagcomp Tag Active))