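; Gameplay attribute component that holds an actor's tag-keyed stats, built on the server from base, threshold and derived-stat DataTables.
; A counter gates the async loads before sending initial data to the client and signalling readiness.
; Instant changes run through a locked queue, while active modifiers recalculate from base by operator and are removable by effect GUID.
; Changed values are clamped, toggle threshold status tags on the owner, broadcast and notify the client.
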(event Custom|SetupAttributesFromDataTable
  (params (DT%20AttributeBaseValues :type Data%20Table%20Soft%20Object%20Reference) (DT%20AttributeThresholds :type Data%20Table%20Soft%20Object%20Reference) (DT%20AttributeDerivedStats :type Data%20Table%20Soft%20Object%20Reference))
  ;[0.15 0.15 0.15 0.5] Initialize the attribute system using provided DataTable
  (Networking|SwitchHasAuthority
    (:Authority
      (CallFunction|InitializeBaseDefinitionData DT%20AttributeBaseValues)
      (CallFunction|InitializeThresholdData DT%20AttributeThresholds)
      (CallFunction|InitializeDerivedData DT%20AttributeDerivedStats))))

(event Custom|InitializeDerivedData
  (params (DT%20AttributeDerivedStats :type Data%20Table%20Soft%20Object%20Reference))
  (bind _output (Utilities|ResolveSoftReference DT%20AttributeDerivedStats))
  ;[0.15 0.15 0.15 0.5] Initialize the attribute system using provided DataTable
  ;;[0.15 0.15 0.15 0.5] Load level-scaled attribute modifiers (derived values) from the Derived DataTable
  (Utilities|AsyncLoadAsset DT%20AttributeDerivedStats
    (:Completed
      (bind _outrownames (DataTable|GetDataTableRowNames _output))
      (for _array_element _outrownames
        (bind _returnvalue (Utilities|GetDataTableRow _output _array_element)
          (:then
            (Utilities|Map|Add (Variables|AttributeSystemDerivedStats|GetAttributeDerivedDefinitionMap) (Utilities|Struct|BreakS_AttributeInitRowDerivedStateValue _returnvalue) _returnvalue))))
      (AttributeSystemLoader|CheckIsAttributeSystemInitialized))))

(event Custom|ReplicateInitAttributeData_CLIENT
  (params (AttributeStates :type Array%20of%20S%20Attribute%20State%20Structures) (AttributeBaseDefinitions :type Array%20of%20S%20Attribute%20Init%20Row%20Base%20Definition%20Structures))
  ;[0.15 0.15 0.15 0.5] Receive initial attribute data from server on client: populate live/base maps and fire notifications for each attribute
  (for _array_element AttributeStates
    (CallFunction|NotifyAttributeChangeCLIENT _array_element))
  (for _array_element_2 AttributeBaseDefinitions
    (Utilities|Map|Add (Variables|Default|GetAttributeDefinitionMap) (.AttributeTag (Utilities|Struct|BreakS_AttributeInitRowBaseDefinition _array_element_2)) _array_element_2)
    (if (GameplayTags|IsGameplayTagValid (.MaxAttributeTag (Utilities|Struct|BreakS_AttributeInitRowBaseDefinition _array_element_2)))
      (Utilities|Map|Add (Variables|Default|GetAttributeDefinitionMap) (.MaxAttributeTag (Utilities|Struct|BreakS_AttributeInitRowBaseDefinition _array_element_2)) _array_element_2))))

(event Custom|NotifyAttributeChange_CLIENT
  (params (AttributeState :type S%20Attribute%20State%20Structure))
  ;[0.15 0.15 0.15 0.5] Handle a single attribute update on the owning client: Cache the new state and broadcast change events
  (AttributeSystemNotifier|BroadcastAttributeChanges AttributeState))

(event Custom|InitAndReplicateLoadedData
  ;[0.15 0.15 0.15 0.5] Initialize the attribute system using provided DataTable
  ;;[0.15 0.15 0.15 0.5] Replicate the freshly initialized attribute data out to connected client
  (bind _values (Utilities|Map|Values (Variables|Default|GetAttributeDefinitionMap)))
  (bind _values_2 (Utilities|Map|Values (Variables|Default|GetAttributeStateMap)))
  (CallFunction|ReplicateInitAttributeDataCLIENT _values_2 _values)
  (for _array_element _values_2
    (AttributeSystemThreshold|UpdateThresholdTagsfromAttribute (.attributetag _array_element)))
  (AttributeSystemLoader|CheckIsAttributeSystemInitialized))

(event Custom|InitializeBaseDefinitionData
  (params (DT%20AttributeBaseValues :type Data%20Table%20Soft%20Object%20Reference))
  (bind _output (Utilities|ResolveSoftReference DT%20AttributeBaseValues))
  ;[0.15 0.15 0.15 0.5] Initialize the attribute system using provided DataTable
  ;;[0.15 0.15 0.15 0.5] Load base attribute start and max values from the Definition DataTable
  (Utilities|AsyncLoadAsset DT%20AttributeBaseValues
    (:Completed
      (bind _outrownames (DataTable|GetDataTableRowNames _output))
      (for _array_element _outrownames
        (bind _returnvalue (Utilities|GetDataTableRow _output _array_element)
          (:then
            (AttributeSystemLoader|RegisterAttributeTag (.AttributeTag (Utilities|Struct|BreakS_AttributeInitRowBaseDefinition _returnvalue)) _returnvalue (.StartValue (Utilities|Struct|BreakS_AttributeInitRowBaseDefinition _returnvalue)))
            (if (GameplayTags|IsGameplayTagValid (.MaxAttributeTag (Utilities|Struct|BreakS_AttributeInitRowBaseDefinition _returnvalue)))
              (AttributeSystemLoader|RegisterAttributeTag (.MaxAttributeTag (Utilities|Struct|BreakS_AttributeInitRowBaseDefinition _returnvalue)) _returnvalue (.BaseValue (Utilities|Struct|BreakS_AttributeInitRowBaseDefinition _returnvalue)))))))
      (AttributeSystemLoader|CheckIsAttributeSystemInitialized))))

(event Custom|InitializeThresholdData
  (params (DT%20AttributeThresholds :type Data%20Table%20Soft%20Object%20Reference))
  (bind _output (Utilities|ResolveSoftReference DT%20AttributeThresholds))
  ;[0.15 0.15 0.15 0.5] Initialize the attribute system using provided DataTable
  ;;[0.15 0.15 0.15 0.5] Load all threshold definitions for status tag checks from the threshold DataTable
  (Utilities|AsyncLoadAsset DT%20AttributeThresholds
    (:Completed
      (bind _outrownames (DataTable|GetDataTableRowNames _output))
      (for _array_element _outrownames
        (bind _returnvalue (Utilities|GetDataTableRow _output _array_element)
          (:then
            (Utilities|Array|Add (Variables|AttributeSystemThreshold|GetAllAttributeThresholdTags) _returnvalue))))
      (AttributeSystemLoader|CheckIsAttributeSystemInitialized))))

(fn RegisterAttributeTag
  (params (AttributeTag :type Gameplay%20Tag%20Structure) (BaseDefinition :type S%20Attribute%20Init%20Row%20Base%20Definition%20Structure) (CurrentValue :type Float%20%28double-precision%29))
  ;[0.15 0.15 0.15 0.5] Register a new attribute: store its base definition and initialize it's live state with the
  ; current value in the component's maps
  (Utilities|Map|Add (Variables|Default|GetAttributeDefinitionMap) AttributeTag BaseDefinition)
  (Utilities|Map|Add (Variables|Default|GetAttributeStateMap) AttributeTag (Utilities|Struct|MakeS_AttributeState AttributeTag CurrentValue)))

(fn BroadcastAttributeChanges
  (params (AttributeState :type S%20Attribute%20State%20Structure))
  (bind _attributetag (Utilities|Struct|BreakS_AttributeState AttributeState))
  ;[0.15 0.15 0.15 0.5] Fetch the updated full attribute state, call the OnAnyAttributeValueChanged delegate, and invoke NotifyAttributes to forward the change to listeners
  (Utilities|Map|Add (Variables|Default|GetAttributeStateMap) _attributetag AttributeState)
  (Default|CallOnAnyAttributeValueChanged (Utilities|Struct|MakeS_AttributeGroupValues _attributetag (AttributeSystemGetter/Setter|GetAttributeValues _attributetag))))

(fn GetAttributeValues
  (params (AttributeTag :type Gameplay%20Tag%20Structure))
  (bind _attributedefinitionmap (Variables|Default|GetAttributeDefinitionMap))
  (bind _value (Utilities|Map|Find _attributedefinitionmap AttributeTag))
  (bind (_attributetag _maxattributetag) (Utilities|Struct|BreakS_AttributeInitRowBaseDefinition _value))
  (if (GameplayTags|IsGameplayTagValid _maxattributetag)
    (return (Utilities|Struct|MakeS_AttributeValues (.CurrentValue (AttributeSystemGetter/Setter|GetAttributeCurrentValue _attributetag)) (.CurrentValue (AttributeSystemGetter/Setter|GetAttributeCurrentValue _maxattributetag)) true))
    (else
      (return (Utilities|Struct|MakeS_AttributeValues (.CurrentValue (AttributeSystemGetter/Setter|GetAttributeCurrentValue AttributeTag)) 0.0 false)))))

(fn GetAttributeCurrentValue
  (params (AttributeTag :type Gameplay%20Tag%20Structure))
  (bind _attributestatemap (Variables|Default|GetAttributeStateMap))
  (bind _value (Utilities|Map|Find _attributestatemap AttributeTag))
  (return (Utilities|Struct|BreakS_AttributeState _value) _value))

(fn SetAttributeInstant
  (params (AttributeTag :type Gameplay%20Tag%20Structure) (ModifierOperator :type E_GE_ModifierOperator%20Enum :default "NewEnumerator0") (EvaluatedValue :type Float%20%28double-precision%29))
  ;[0.15 0.15 0.15 0.5] Helper function
  ; Create and enqueue a resolved modifier for the specified attribute, operator, and evaluated value
  (AttributeSystemModification|AddQueueModifier (Utilities|Array|MakeArray (Utilities|Struct|MakeS_AttributeResolvedModifier "00000000000000000000000000000000" "00000000000000000000000000000000" AttributeTag ModifierOperator EvaluatedValue))))

(fn AddQueueModifier
  (params (Modifiers :type Array%20of%20S%20Attribute%20Resolved%20Modifier%20Structures))
  (Utilities|Array|AppendArray (Variables|AttributeSystemModification|GetQueuedModifiers) Modifiers)
  (AttributeSystemModification|ProcessNextQueuedModifiers))

(fn RecalculateModifiersDirectly
  (params (Modifiers :type Array%20of%20S%20Attribute%20Resolved%20Modifier%20Structures))
  ;[0.15 0.15 0.15 0.5] Immediately apply every modifier in the list to the live attribute states without waiting for the queue
  (for _array_element Modifiers
    (bind _clampedattributestate (AttributeSystemModification|ClampAttributeValue (.AttributeTag (Utilities|Struct|BreakS_AttributeResolvedModifier _array_element)) (Utilities|Select :Index (.ModifierOperator (Utilities|Struct|BreakS_AttributeResolvedModifier _array_element)) :NewEnumerator0 (+ (.CurrentValue (AttributeSystemGetter/Setter|GetAttributeCurrentValue (.AttributeTag (Utilities|Struct|BreakS_AttributeResolvedModifier _array_element)))) (.EvaluatedValue (Utilities|Struct|BreakS_AttributeResolvedModifier _array_element))) :NewEnumerator1 (* (.CurrentValue (AttributeSystemGetter/Setter|GetAttributeCurrentValue (.AttributeTag (Utilities|Struct|BreakS_AttributeResolvedModifier _array_element)))) (+ 1.0 (.EvaluatedValue (Utilities|Struct|BreakS_AttributeResolvedModifier _array_element)))) :NewEnumerator2 (Math|Float|SafeDivide (.CurrentValue (AttributeSystemGetter/Setter|GetAttributeCurrentValue (.AttributeTag (Utilities|Struct|BreakS_AttributeResolvedModifier _array_element)))) (.EvaluatedValue (Utilities|Struct|BreakS_AttributeResolvedModifier _array_element))) :NewEnumerator3 (.EvaluatedValue (Utilities|Struct|BreakS_AttributeResolvedModifier _array_element)))))
    (AttributeSystemModification|SetAttributeStateValue _clampedattributestate)))

(fn ClampAttributeValue
  (params (AttributeTag :type Gameplay%20Tag%20Structure) (NewCurrentValue :type Float%20%28double-precision%29))
  (bind _attributedefinitionmap (Variables|Default|GetAttributeDefinitionMap))
  (bind _value (Utilities|Map|Find _attributedefinitionmap AttributeTag))
  (bind (_maxattributetag _minvalue _maxvalue _clampbymaxattributevalue) (Utilities|Struct|BreakS_AttributeInitRowBaseDefinition _value))
  ;[0.15 0.15 0.15 0.5] Look up the attribute's confugured min/max, then clamp the current value within that range before returning it
  (if (and (GameplayTags|IsGameplayTagValid _maxattributetag) _clampbymaxattributevalue)
    (return (Utilities|Struct|MakeS_AttributeState AttributeTag (Math|Float|Clamp(Float) NewCurrentValue _minvalue (.CurrentValue (AttributeSystemGetter/Setter|GetAttributeCurrentValue _maxattributetag)))))
    (else
      (return (Utilities|Struct|MakeS_AttributeState AttributeTag (Math|Float|Clamp(Float) NewCurrentValue _minvalue _maxvalue))))))

(fn SetAttributeStateValue
  (params (AttributeState :type S%20Attribute%20State%20Structure))
  (bind _attributetag (Utilities|Struct|BreakS_AttributeState AttributeState))
  ;[0.15 0.15 0.15 0.5] Write the new live state into the map, update threshold tags, broadcast change events, and notify the owning client
  (Utilities|Map|Add (Variables|Default|GetAttributeStateMap) _attributetag AttributeState)
  (AttributeSystemThreshold|UpdateThresholdTagsfromAttribute _attributetag)
  (AttributeSystemNotifier|BroadcastAttributeChanges AttributeState)
  (CallFunction|NotifyAttributeChangeCLIENT AttributeState))

(fn ProcessNextQueuedModifiers
  ;[0.15 0.15 0.15 0.5] Ensure only one modifier is processed at a time by locking the queue, storing the current modifier, removing it safely, and then executing it.
  (if (not (or (Variables|AttributeSystemModification|GetIsProcessingModifierQueue) (Utilities|Array|IsEmpty (Variables|AttributeSystemModification|GetQueuedModifiers))))
    (Variables|AttributeSystemModification|SetIsProcessingModifierQueue true)
    (bind _output_get (LocalVariables|SetToExecuteModifiers (Variables|AttributeSystemModification|GetQueuedModifiers)))
    (Utilities|Array|Clear (Variables|AttributeSystemModification|GetQueuedModifiers))
    (AttributeSystemModification|RecalculateModifiersDirectly _output_get)
    (Variables|AttributeSystemModification|SetIsProcessingModifierQueue false)
    (AttributeSystemModification|ProcessNextQueuedModifiers)))

(fn UpdateThresholdTagsfromAttribute
  (params (AttributeTag :type Gameplay%20Tag%20Structure))
  ;[0.15 0.15 0.15 0.5] Loop through each threshold definition, compare the attribute's
  ; live value against its configured min/max, and add or remove the corresponding status tags
  (for _array_element (Variables|AttributeSystemThreshold|GetAllAttributeThresholdTags)
    (if (Utilities|Array|ContainsItem (AttributeSystemGetter/Setter|GetAttributeGroupTags AttributeTag) (.AttributeTagCurrentValue (Utilities|Struct|BreakS_AttributeThresholdTag _array_element)))
      (if (and (>= (Utilities|Select :Index (.ThresholdType (Utilities|Struct|BreakS_AttributeThresholdTag _array_element)) :NewEnumerator0 (Math|Float|SafeDivide (.current (AttributeSystemGetter/Setter|GetAttributeValues (.AttributeTagCurrentValue (Utilities|Struct|BreakS_AttributeThresholdTag _array_element)))) (.max (AttributeSystemGetter/Setter|GetAttributeValues (.AttributeTagCurrentValue (Utilities|Struct|BreakS_AttributeThresholdTag _array_element))))) :NewEnumerator1 (.current (AttributeSystemGetter/Setter|GetAttributeValues (.AttributeTagCurrentValue (Utilities|Struct|BreakS_AttributeThresholdTag _array_element))))) (.MinValue (Utilities|Struct|BreakS_AttributeThresholdTag _array_element))) (<= (Utilities|Select :Index (.ThresholdType (Utilities|Struct|BreakS_AttributeThresholdTag _array_element)) :NewEnumerator0 (Math|Float|SafeDivide (.current (AttributeSystemGetter/Setter|GetAttributeValues (.AttributeTagCurrentValue (Utilities|Struct|BreakS_AttributeThresholdTag _array_element)))) (.max (AttributeSystemGetter/Setter|GetAttributeValues (.AttributeTagCurrentValue (Utilities|Struct|BreakS_AttributeThresholdTag _array_element))))) :NewEnumerator1 (.current (AttributeSystemGetter/Setter|GetAttributeValues (.AttributeTagCurrentValue (Utilities|Struct|BreakS_AttributeThresholdTag _array_element))))) (.MaxValue (Utilities|Struct|BreakS_AttributeThresholdTag _array_element))))
        (bind _result (Class|BPIAbilitySystemProvider|HasGameplayTag(Message) (Components|GetOwner) (.TagToAdd (Utilities|Struct|BreakS_AttributeThresholdTag _array_element))))
        (if (not _result)
          (Class|BPIAbilitySystemProvider|SetGameplayTag(Message) (Components|GetOwner) (.TagToAdd (Utilities|Struct|BreakS_AttributeThresholdTag _array_element)) true))
        (else
          (bind _result_2 (Class|BPIAbilitySystemProvider|HasGameplayTag(Message) (Components|GetOwner) (.TagToAdd (Utilities|Struct|BreakS_AttributeThresholdTag _array_element))))
          (if _result_2
            (Class|BPIAbilitySystemProvider|SetGameplayTag(Message) (Components|GetOwner) (.TagToAdd (Utilities|Struct|BreakS_AttributeThresholdTag _array_element)) false)))))))

(fn GetAttributeGroupTags
  (params (AttributeTag :type Gameplay%20Tag%20Structure))
  (bind _attributedefinitionmap (Variables|Default|GetAttributeDefinitionMap))
  (bind _value (Utilities|Map|Find _attributedefinitionmap AttributeTag))
  (bind (_attributetag _maxattributetag) (Utilities|Struct|BreakS_AttributeInitRowBaseDefinition _value))
  (return (select (GameplayTags|IsGameplayTagValid _maxattributetag) (Utilities|Array|MakeArray _attributetag _maxattributetag) (Utilities|Array|MakeArray _attributetag))))

(fn AddModifierstoAttribute
  (params (Modifiers :type Array%20of%20S%20Attribute%20Resolved%20Modifier%20Structures))
  ;[0.15 0.15 0.15 0.5] For each resolved modifier, insert it into the active modifier list and group by operator type before triggering a recalculation
  (for _array_element Modifiers
    (bind _output_get (LocalVariables|SetNewModifiersGroup (.Value (Utilities|Map|Find (Variables|AttributeSystemModification|GetActiveAttributeModifiers) (.AttributeTag (Utilities|Struct|BreakS_AttributeResolvedModifier _array_element))))))
    (Utilities|FlowControl|Sequence
      (:then_0
        (switch Utilities|FlowControl|Switch|SwitchonE_GE_ModifierOperator (.ModifierOperator (Utilities|Struct|BreakS_AttributeResolvedModifier _array_element))
          (:NewEnumerator0
            (Utilities|Array|AddUnique (.AddModifiers (Utilities|Struct|BreakS_AttributeModifiersOperatorGroup _output_get)) _array_element))
          (:NewEnumerator1
            (Utilities|Array|AddUnique (.MultiplyModifiers (Utilities|Struct|BreakS_AttributeModifiersOperatorGroup _output_get)) _array_element))
          (:NewEnumerator2
            (Utilities|Array|AddUnique (.DivideModifiers (Utilities|Struct|BreakS_AttributeModifiersOperatorGroup _output_get)) _array_element))
          (:NewEnumerator3
            (Utilities|Struct|SetmembersinS_AttributeModifiersOperatorGroup (LocalVariables|GetNewModifiersGroup) (Utilities|Array|MakeArray _array_element)))))
      (:then_1
        (Utilities|Array|AddUnique (LocalVariables|GetModifiedAttributeTags) (.AttributeTag (Utilities|Struct|BreakS_AttributeResolvedModifier _array_element)))
        (Utilities|Map|Add (Variables|AttributeSystemModification|GetActiveAttributeModifiers) (.AttributeTag (Utilities|Struct|BreakS_AttributeResolvedModifier _array_element)) (LocalVariables|GetNewModifiersGroup)))))
  (for _array_element_2 (LocalVariables|GetModifiedAttributeTags)
    (AttributeSystemModification|RecalculateAttribute _array_element_2)))

(fn RecalculateAttribute
  (params (AttributeTag :type Gameplay%20Tag%20Structure))
  (bind _activeattributemodifiers (Variables|AttributeSystemModification|GetActiveAttributeModifiers))
  (bind (_value _returnvalue) (Utilities|Map|Find _activeattributemodifiers AttributeTag))
  (bind (_overridemodifiers _addmodifiers _multiplymodifiers _dividemodifiers) (Utilities|Struct|BreakS_AttributeModifiersOperatorGroup _value))
  ;[0.15 0.15 0.15 0.5] Compute the final attribute value by summing base value and all modifiers, clamp it within valid bounds, and update the live state
  (if _returnvalue
    (bind _clampedattributestate (AttributeSystemModification|ClampAttributeValue AttributeTag (Math|Float|SafeDivide (* (+ (select (Utilities|Array|IsNotEmpty _overridemodifiers) (AttributeSystemModification|SumModifiersValues _overridemodifiers) (AttributeSystemGetter/Setter|GetAttributeBaseValue AttributeTag)) (AttributeSystemModification|SumModifiersValues _addmodifiers)) (+ 1.0 (AttributeSystemModification|SumModifiersValues _multiplymodifiers))) (+ 1.0 (AttributeSystemModification|SumModifiersValues _dividemodifiers)))))
    (AttributeSystemModification|SetAttributeStateValue _clampedattributestate)))

(fn SumModifiersValues
  (params (Modifiers :type Array%20of%20S%20Attribute%20Resolved%20Modifier%20Structures))
  ;[0.15 0.15 0.15 0.5] Interate all resolved modifiers for an attribute and sum their evaluated values into a single total
  (for _array_element Modifiers
    (LocalVariables|SetTempSum (+ (LocalVariables|GetTempSum) (Utilities|Struct|BreakS_AttributeResolvedModifier _array_element))))
  (return (LocalVariables|GetTempSum)))

(fn GetAttributeBaseValue
  (params (AttributeTag :type Gameplay%20Tag%20Structure))
  ;[0.15 0.15 0.15 0.5] Returns a attribute BaseValue matching the given gameplay tag
  (return (Utilities|Struct|BreakS_AttributeInitRowBaseDefinition (.Value (Utilities|Map|Find (Variables|Default|GetAttributeDefinitionMap) AttributeTag)))))

(fn RemoveModifiersfromAttribute
  (params (GameplayEffectGUID :type Guid%20Structure))
  ;[0.15 0.15 0.15 0.5] Find and remove modifiers matching the given gameplay effect GUID from all active modifier lists, returning whether any were removed
  (bind _keys (Utilities|Map|Keys (Variables|AttributeSystemModification|GetActiveAttributeModifiers)))
  (for _array_element _keys
    (bind _output_get (LocalVariables|SetModifierGroups (.Value (Utilities|Map|Find (Variables|AttributeSystemModification|GetActiveAttributeModifiers) _array_element))))
    (LocalVariables|SetIsModifier false)
    (Utilities|FlowControl|Sequence
      (:then_0
        (bind (_ismodified _newmodifiers) (AttributeSystemModification|RemoveModifiersbyEffectGUID (.OverrideModifiers (Utilities|Struct|BreakS_AttributeModifiersOperatorGroup _output_get)) GameplayEffectGUID))
        (if _ismodified
          (Utilities|Struct|SetmembersinS_AttributeModifiersOperatorGroup (LocalVariables|GetModifierGroups) _newmodifiers)
          (LocalVariables|SetIsModifier true)))
      (:then_1
        (bind (_ismodified_2 _newmodifiers_2) (AttributeSystemModification|RemoveModifiersbyEffectGUID (.AddModifiers (Utilities|Struct|BreakS_AttributeModifiersOperatorGroup _output_get)) GameplayEffectGUID))
        (if _ismodified_2
          (Utilities|Struct|SetmembersinS_AttributeModifiersOperatorGroup (LocalVariables|GetModifierGroups) _newmodifiers_2)
          (LocalVariables|SetIsModifier true)))
      (:then_2
        (bind (_ismodified_3 _newmodifiers_3) (AttributeSystemModification|RemoveModifiersbyEffectGUID (.MultiplyModifiers (Utilities|Struct|BreakS_AttributeModifiersOperatorGroup _output_get)) GameplayEffectGUID))
        (if _ismodified_3
          (Utilities|Struct|SetmembersinS_AttributeModifiersOperatorGroup (LocalVariables|GetModifierGroups) _newmodifiers_3)
          (LocalVariables|SetIsModifier true)))
      (:then_3
        (bind (_ismodified_4 _newmodifiers_4) (AttributeSystemModification|RemoveModifiersbyEffectGUID (.DivideModifiers (Utilities|Struct|BreakS_AttributeModifiersOperatorGroup _output_get)) GameplayEffectGUID))
        (if _ismodified_4
          (Utilities|Struct|SetmembersinS_AttributeModifiersOperatorGroup (LocalVariables|GetModifierGroups) _newmodifiers_4)
          (LocalVariables|SetIsModifier true)))
      (:then_4
        (if (LocalVariables|GetIsModifier)
          (Utilities|Map|Add (Variables|AttributeSystemModification|GetActiveAttributeModifiers) _array_element (LocalVariables|GetModifierGroups))
          (AttributeSystemModification|RecalculateAttribute _array_element))))))

(fn RemoveModifiersbyEffectGUID
  (params (ResolvedModifiers :type Array%20of%20S%20Attribute%20Resolved%20Modifier%20Structures) (GameplayEffectGUID :type Guid%20Structure))
  ;[0.15 0.15 0.15 0.5] Filter a specific attribute's list by GUID, update the list and operator grounds, and flag the attribute for recalculation
  (LocalVariables|SetModifiers ResolvedModifiers)
  (for _array_element ResolvedModifiers
    (if (== GameplayEffectGUID (Utilities|Struct|BreakS_AttributeResolvedModifier _array_element))
      (Utilities|Array|RemoveItem (LocalVariables|GetModifiers) _array_element)
      (LocalVariables|SetFound true)))
  (return (LocalVariables|GetFound) (LocalVariables|GetModifiers)))

(fn GetAttributeDerivedDefinition
  (params (AttributeDerivedTag :type Gameplay%20Tag%20Structure))
  (bind _attributederiveddefinitionmap (Variables|AttributeSystemDerivedStats|GetAttributeDerivedDefinitionMap))
  (bind (_value _returnvalue) (Utilities|Map|Find _attributederiveddefinitionmap AttributeDerivedTag))
  (bind (_modifierratetype _valuesbylevel) (Utilities|Struct|BreakS_AttributeInitRowDerivedStateValue _value))
  (if _returnvalue
    (return _modifierratetype (Utilities|Array|Get(acopy) _valuesbylevel))
    (else
      (CallFunction|PrintError "Attribute derived stat not found for derivedTag:" (Utilities|String|ToString(Name) (GameplayTags|GetTagName AttributeDerivedTag)) true)
      (return "NewEnumerator0" 0.0))))

(fn GetAllAttributeTags
  (bind _keys (Utilities|Map|Keys (Variables|Default|GetAttributeStateMap)))
  (return (GameplayTags|MakeGameplayTagContainerfromArray _keys)))

(fn CheckIsAttributeSystemInitialized
  ;[0.15 0.15 0.15 0.5] Increment the async-load counter. Once all tables are loaded, initialize and replicate the loaded data, then mark the Attribute System ready and fire the ready event.
  (bind _result (Math|Integer|IncrementInt (Variables|AttributeSystemLoader|GetAsyncLoadCounter))
    (:%20%20
      (bind _output_get (Variables|AttributeSystemLoader|SetIsComponentInitialized (>= _result 4)))
      (if _output_get
        (Default|CallOnAttributeSystemIsReady)
        (elif (>= _result 3)
          (CallFunction|InitandReplicateLoadedData))))))

(fn IsAttributeComponentReady
  (return (Variables|AttributeSystemLoader|GetIsComponentInitialized)))