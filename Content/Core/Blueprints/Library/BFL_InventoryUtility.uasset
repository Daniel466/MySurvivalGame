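; Blueprint function library of inventory slot helpers for checking, building and weighing item slots.
; Empty and contained-item checks test whether the slot's soft data asset references are valid.
; MakeItemToAdd resolves a soft item data reference into a new slot with ID, quantity, default durability and weight, printing an error if resolution fails.
; Slot weight is quantity times per-item weight.
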(fn IsSlotEmpty
  (params (Slot :type S%20Inventory%20Slot%20Structure))
  (return (not (Utilities|IsValidSoftObjectReference (.ItemDataAsset (Utilities|Struct|BreakS_InventorySlot Slot))))))

(fn IsSlotNotEmpty
  (params (Slot :type S%20Inventory%20Slot%20Structure))
  (return (not (BFLInventoryUtility|IsSlotEmpty Slot))))

(fn MakeItemtoAdd
  (params (ItemDataSoftObject :type PDA%20Item%20Data%20Soft%20Object%20Reference) (Quantity :type Integer))
  (bind _itemdataasset (CallFunction|ResolveSoftItemDataReference ItemDataSoftObject))
  (Utilities|IsValid _itemdataasset
    (:Is%20Valid
      (return (Utilities|Struct|MakeS_InventorySlot (Variables|/Game/Core/DataAssets/PrimaryAssets/PDA_ItemData.PDA_ItemData_C|GetItemID _itemdataasset) Quantity 0 ItemDataSoftObject (Default|GetDefaultDurability _itemdataasset) (Default|GetDefaultDurability _itemdataasset) (Variables|/Game/Core/DataAssets/PrimaryAssets/PDA_ItemData.PDA_ItemData_C|GetItemWeight _itemdataasset) "(CurrentAmount_6_DDA7B116471BD50C919293AF096477D4=0.000000,MaxCapacity_8_CC4429FB4AADF67EE1592095CB6D3DD2=0.000000,ContainedItemDataAsset_11_BA22AE7648D9C485604934A63989E593=None)" 0)))
    (:Is%20Not%20Valid
      (Development|PrintString 0 "Can't resolve ItemDataAsset"))))

(fn GetSlotWeight
  (params (Slot :type S%20Inventory%20Slot%20Structure))
  (bind (_quantity _itemweight) (Utilities|Struct|BreakS_InventorySlot Slot))
  (return (* _quantity _itemweight)))

(fn HasSlotContainedItem
  (params (Slot :type S%20Inventory%20Slot%20Structure))
  (return (Utilities|IsValidSoftObjectReference (Utilities|Struct|BreakS_SlotContainedItem (Utilities|Struct|BreakS_InventorySlot Slot)))))