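; Camera Director for the player character that picks which Gameplay Camera rigs to activate each evaluation.
; It reads camera properties from the owning Character through a GetPropertiesForCameraMessage call.
; Camera mode selects the strafe, aim or weapon-aim rig proxy, then a crouch stance separately activates a crouch offset rig on top.
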(event EventRunCameraDirector
  (params (Params :type Blueprint%20Camera%20Director%20Evaluation%20Params%20Structure%20%28by%20ref%29))
  (bind _returnvalue (Class|BPICharacter|GetPropertiesforCamera(Message) (Class|BlueprintCameraDirectorEvaluator|FindEvaluationContextOwnerActor "/Script/Engine.Character")))
  (Variables|Default|SetPropertiesCamera _returnvalue)
  (Utilities|FlowControl|Sequence
    (:then_0
      (switch Utilities|FlowControl|Switch|SwitchonE_CameraMode (.CameraMode (Utilities|Struct|BreakS_CharacterCameraProperties (Variables|Default|GetPropertiesCamera)))
        (:NewEnumerator0
          (Class|BlueprintCameraDirectorEvaluator|ActivateCameraRigViaProxy "/Game/Core/Blueprints/Gameplay/Cameras/CRIGProxy_StrafeCamera.CRIGProxy_StrafeCamera"))
        (:NewEnumerator1
          (Class|BlueprintCameraDirectorEvaluator|ActivateCameraRigViaProxy "/Game/Core/Blueprints/Gameplay/Cameras/CRIGProxy_Aim.CRIGProxy_Aim"))
        (:NewEnumerator2
          (Class|BlueprintCameraDirectorEvaluator|ActivateCameraRigViaProxy "/Game/Core/Blueprints/Gameplay/Cameras/CRIGProxy_AimWeapon.CRIGProxy_AimWeapon"))))
    (:then_1
      (switch Utilities|FlowControl|Switch|SwitchonE_MovementStance (.Stance (Utilities|Struct|BreakS_CharacterCameraProperties (Variables|Default|GetPropertiesCamera)))
        (:NewEnumerator1
          (Class|BlueprintCameraDirectorEvaluator|ActivateCameraRigViaProxy "/Game/Core/Blueprints/Gameplay/Cameras/CRIGProxy_CrouchOffset.CRIGProxy_CrouchOffset"))))))